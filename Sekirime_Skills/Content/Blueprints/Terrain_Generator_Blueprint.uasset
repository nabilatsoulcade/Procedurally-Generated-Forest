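; Terrain generator actor that builds a procedural grass-textured ground mesh with collision and randomly varied height.
; It creates a welded grid from width, height and spacing settings, then offsets each vertex's Z randomly within the variance range.
; The mesh section and material are reapplied inside the per-vertex loop.
; The construction script offers a flat-plane debug mode, while BeginPlay always generates randomized terrain.
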(event `self.ReceiveBeginPlay`
  (bind (_triangles _vertices _uvs) (`KismetProceduralMeshLibrary.CreateGridMeshWelded` (`self.TerrainWidth`) (`self.TerrainHeight`) (`KismetMathLibrary.Conv_IntToDouble` (`self.TerrainGridSpacing`))))
  (for (_array_element _array_index) _vertices
    (`KismetArrayLibrary.Array_Set` _vertices _array_index (`KismetMathLibrary.MakeVector` (.x _array_element) (.y _array_element) (+ (`KismetMathLibrary.RandomFloatInRange` (`self.TerrainVarianceMin`) (`self.TerrainVarianceMax`)) (.z _array_element))))
    (`ProceduralMeshComponent.CreateMeshSection_LinearColor` :`self` (`self.ProceduralMesh`) :`Vertices` _vertices :`Triangles` _triangles :`UV0` _uvs :`bCreateCollision` true)
    (`PrimitiveComponent.SetMaterial` (`self.ProceduralMesh`) 0 "/Game/StarterContent/Materials/M_Ground_Grass.M_Ground_Grass")))

(fn `UserConstructionScript`
  (if (`self.TerrainDebugMode`)
    (bind (_triangles _vertices _uvs) (`KismetProceduralMeshLibrary.CreateGridMeshWelded` (`self.TerrainWidth`) (`self.TerrainHeight`) (`KismetMathLibrary.Conv_IntToDouble` (`self.TerrainGridSpacing`))))
    (`ProceduralMeshComponent.CreateMeshSection_LinearColor` :`self` (`self.ProceduralMesh`) :`Vertices` _vertices :`Triangles` _triangles :`UV0` _uvs :`bCreateCollision` true)
    (`PrimitiveComponent.SetMaterial` (`self.ProceduralMesh`) 0 "/Game/StarterContent/Materials/M_Ground_Grass.M_Ground_Grass")
    (else
      (bind (_triangles_2 _vertices_2 _uvs_2) (`KismetProceduralMeshLibrary.CreateGridMeshWelded` (`self.TerrainWidth`) (`self.TerrainHeight`) (`KismetMathLibrary.Conv_IntToDouble` (`self.TerrainGridSpacing`))))
      (for (_array_element _array_index) _vertices_2
        (`KismetArrayLibrary.Array_Set` _vertices_2 _array_index (`KismetMathLibrary.MakeVector` (.x _array_element) (.y _array_element) (+ (`KismetMathLibrary.RandomFloatInRange` (`self.TerrainVarianceMin`) (`self.TerrainVarianceMax`)) (.z _array_element))))
        (`ProceduralMeshComponent.CreateMeshSection_LinearColor` :`self` (`self.ProceduralMesh`) :`Vertices` _vertices_2 :`Triangles` _triangles_2 :`UV0` _uvs_2 :`bCreateCollision` true)
        (`PrimitiveComponent.SetMaterial` (`self.ProceduralMesh`) 0 "/Game/StarterContent/Materials/M_Ground_Grass.M_Ground_Grass")))))